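; bOOM is a Paper2D Blueprint that plays one-shot animated cutscenes with sound, apparently game endings: shelter explosion, crateman, bear, raiders and tetanus.
; On BeginPlay it stops its flipbook and disables looping.
; Each custom event swaps in its flipbook, plays it from the start and fires a 2D sound.
; Explosion and bear sounds use delays to sync, while raid and tetanus sounds start partway through at reduced volume.
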(event Custom|PlayExplode
  (bind _paperflipbook (Variables|Default|GetPaperFlipbook))
  (Sprite|SetFlipbook _paperflipbook "/Game/HUD/EndingAnims/Selfdestruct/Boom_boom_shelter_sprite_sheet_with_extra_frames1.Boom_boom_shelter_sprite_sheet_with_extra_frames1")
  (Components|Timeline|PlayfromStart _paperflipbook)
  (Utilities|FlowControl|Delay 1.0)
  (Audio|PlaySound2D "/Game/Sounds/explosion-42132.explosion-42132" 1.0 1.0 0.0 0 0))

(event Custom|PlayCrate
  (bind _paperflipbook (Variables|Default|GetPaperFlipbook))
  (Sprite|SetFlipbook _paperflipbook "/Game/HUD/EndingAnims/Crateman/crateman_ending1.crateman_ending1")
  (Components|Timeline|PlayfromStart _paperflipbook)
  (Audio|PlaySound2D "/Game/Sounds/3-legged-robot-walker-86726.3-legged-robot-walker-86726" 1.0 1.0 5.0 0 0))

(event Custom|PlayBear
  (bind _paperflipbook (Variables|Default|GetPaperFlipbook))
  (Sprite|SetFlipbook _paperflipbook "/Game/HUD/EndingAnims/Bear/bear_with_him1.bear_with_him1")
  (Components|Timeline|PlayfromStart _paperflipbook)
  (Utilities|FlowControl|Delay 2.0)
  (Audio|PlaySound2D "/Game/Sounds/bear-191995.bear-191995" 1.0 1.0 0.0 0 0))

(event Custom|raid
  (bind _paperflipbook (Variables|Default|GetPaperFlipbook))
  (Sprite|SetFlipbook _paperflipbook "/Game/HUD/EndingAnims/raiders/RaidersPLEEEEEASE_WORK1.RaidersPLEEEEEASE_WORK1")
  (Components|Timeline|PlayfromStart _paperflipbook)
  (Audio|PlaySound2D "/Game/Sounds/siren-alert-96052.siren-alert-96052" 0.8 1.0 4.0 0 0))

(event Custom|tenatus
  (bind _paperflipbook (Variables|Default|GetPaperFlipbook))
  (Sprite|SetFlipbook _paperflipbook "/Game/HUD/EndingAnims/megatanatus/mega_tetnas_ending1.mega_tetnas_ending1")
  (Components|Timeline|PlayfromStart _paperflipbook)
  (Audio|PlaySound2D "/Game/Sounds/metal-door-creaking-closing-47323.metal-door-creaking-closing-47323" 0.5 1.0 1.0 0 0))

(event EventBeginPlay
  (bind _paperflipbook (Variables|Default|GetPaperFlipbook))
  (Audio|Components|Audio|Stop _paperflipbook)
  (Components|Timeline|SetLooping _paperflipbook false))

(event Collision|EventActorBeginOverlap
  (params (OtherActor :type Actor%20Object%20Reference)))

(event EventTick
  (params (DeltaSeconds :type Float%20%28single-precision%29)))

(fn ConstructionScript)